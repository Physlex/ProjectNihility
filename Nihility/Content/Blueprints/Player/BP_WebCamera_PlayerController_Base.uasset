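; Base player controller that moves the view between level cameras through a WebCameraManager in response to directional input.
; On BeginPlay it registers every CameraActor in the scene with the manager.
; Four input actions each fire a key-press event, request a directional transition from the manager, and call SetViewTargetWithBlend on any valid result.
; AssignRoot sets the view to the manager's root camera but is not called within this graph.
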(event `self.ReceiveBeginPlay`
  ;[1 1 1] Allocate Actors in Scene
  (bind _outactors (`GameplayStatics.GetAllActorsOfClass` "/Script/Engine.CameraActor"))
  (for _array_element _outactors
    (`/Engine/EditorBlueprintResources/StandardMacros.IsValid` _array_element
      (:`Is Valid`
        (`WebCamM.appendCamera` (`self.Web Camera Manager`) _array_element))
      (:`Is Not Valid`
        (`KismetSystemLibrary.PrintString` "Error: Invalid Camera Actor" true true (struct :`G` 0.66 :`B` 1.0 :`A` 1.0) 5.0))))
  (`KismetSystemLibrary.PrintString` "Camera-append-loop completed"))

(event `EnhancedInput|/Game/Input/MouseAndKeyboard/IA_transition_camera_forward`
  (params (ActionValue :type Boolean) (ElapsedSeconds :type "Float (double-precision)") (TriggeredSeconds :type "Float (double-precision)") (InputAction :type "InputAction Object Reference" :default "/Game/Input/MouseAndKeyboard/IA_transition_camera_forward.IA_transition_camera_forward"))
  ;[1 1 1] Forward Key Press
  (:`Triggered`
    (`self.Event_ForwardKeyPress`)
    ;[1 1 1] Camera Transition Event Coordination
    (bind _returnvalue (`WebCamM.transition` (`self.Web Camera Manager`) "up"))
    (`/Engine/EditorBlueprintResources/StandardMacros.IsValid` _returnvalue
      (:`Is Valid`
        (`self.SetViewTargetWithBlend` _returnvalue)))))

(event `EnhancedInput|/Game/Input/MouseAndKeyboard/IA_transition_camera_backwards`
  (params (ActionValue :type Boolean) (ElapsedSeconds :type "Float (double-precision)") (TriggeredSeconds :type "Float (double-precision)") (InputAction :type "InputAction Object Reference" :default "/Game/Input/MouseAndKeyboard/IA_transition_camera_backwards.IA_transition_camera_backwards"))
  ;[1 1 1] Backward Key Press
  (:`Triggered`
    (`self.Event_BackwardsKeyPress`)
    ;[1 1 1] Camera Transition Event Coordination
    (bind _returnvalue (`WebCamM.transition` (`self.Web Camera Manager`) "down"))
    (`/Engine/EditorBlueprintResources/StandardMacros.IsValid` _returnvalue
      (:`Is Valid`
        (`self.SetViewTargetWithBlend` _returnvalue)))))

(event `EnhancedInput|/Game/Input/MouseAndKeyboard/IA_transition_camera_left`
  (params (ActionValue :type Boolean) (ElapsedSeconds :type "Float (double-precision)") (TriggeredSeconds :type "Float (double-precision)") (InputAction :type "InputAction Object Reference" :default "/Game/Input/MouseAndKeyboard/IA_transition_camera_left.IA_transition_camera_left"))
  ;[1 1 1] Left Key Press
  (:`Triggered`
    (`self.Event_LeftKeyPress`)
    ;[1 1 1] Camera Transition Event Coordination
    (bind _returnvalue (`WebCamM.transition` (`self.Web Camera Manager`) "left"))
    (`/Engine/EditorBlueprintResources/StandardMacros.IsValid` _returnvalue
      (:`Is Valid`
        (`self.SetViewTargetWithBlend` _returnvalue)))))

(event `EnhancedInput|/Game/Input/MouseAndKeyboard/IA_transition_camera_right`
  (params (ActionValue :type Boolean) (ElapsedSeconds :type "Float (double-precision)") (TriggeredSeconds :type "Float (double-precision)") (InputAction :type "InputAction Object Reference" :default "/Game/Input/MouseAndKeyboard/IA_transition_camera_right.IA_transition_camera_right"))
  ;[1 1 1] Right Key Press
  (:`Triggered`
    (`self.Event_RightKeyPress`)
    ;[1 1 1] Camera Transition Event Coordination
    (bind _returnvalue (`WebCamM.transition` (`self.Web Camera Manager`) "right"))
    (`/Engine/EditorBlueprintResources/StandardMacros.IsValid` _returnvalue
      (:`Is Valid`
        (`self.SetViewTargetWithBlend` _returnvalue)))))

(fn `AssignRoot`
  ;[1 1 1] Set First View Target
  (bind _returnvalue (`WebCamM.getRootCamera` (`self.Web Camera Manager`)))
  (`/Engine/EditorBlueprintResources/StandardMacros.IsValid` _returnvalue
    (:`Is Valid`
      (`self.SetViewTargetWithBlend` _returnvalue))
    (:`Is Not Valid`
      (`KismetSystemLibrary.PrintString` "Root Camera Invalid" true true (struct :`G` 0.66 :`B` 1.0 :`A` 1.0) 10.0))))

(fn `UserConstructionScript`)