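; Player controller that sets up a network of linked scene cameras and views the game through the root one.
; On BeginPlay it appends every valid CameraActor to its WebCameraManager, then links them by index with hardcoded left/right connections, forming a three-camera chain.
; It then sets the manager's root camera as the view target, printing debug messages for progress and invalid cameras.
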(event `self.ReceiveBeginPlay`
  (bind _web_camera_manager (`self.Web Camera Manager`))
  ;[1 1 1] Allocate Actors in Scene
  (bind _outactors (`GameplayStatics.GetAllActorsOfClass` "/Script/Engine.CameraActor"))
  (for _array_element _outactors
    (`/Engine/EditorBlueprintResources/StandardMacros.IsValid` _array_element
      (:`Is Valid`
        (`WebCamM.appendCamera` (`self.Web Camera Manager`) _array_element))
      (:`Is Not Valid`
        (`KismetSystemLibrary.PrintString` "Error: Invalid Camera Actor" true true (struct :`G` 0.66 :`B` 1.0 :`A` 1.0) 5.0))))
  (`KismetSystemLibrary.PrintString` "Camera-append-loop completed")
  ;[1 1 1] This is where most of the scripting of the camera system is based around. Every camera must have each tra
  (`WebCamM.connectCamerasByType` _web_camera_manager 0 1 "right")
  (`WebCamM.connectCamerasByType` _web_camera_manager 1 0 "left")
  (`WebCamM.connectCamerasByType` _web_camera_manager 1 2 "right")
  (`WebCamM.connectCamerasByType` _web_camera_manager 2 1 "left")
  ;[1 1 1] Set First View Target
  (bind _returnvalue (`WebCamM.getRootCamera` (`self.Web Camera Manager`)))
  (`/Engine/EditorBlueprintResources/StandardMacros.IsValid` _returnvalue
    (:`Is Valid`
      (`self.SetViewTargetWithBlend` _returnvalue))
    (:`Is Not Valid`
      (`KismetSystemLibrary.PrintString` "Root Camera Invalid" true true (struct :`G` 0.66 :`B` 1.0 :`A` 1.0) 10.0))))

(fn `UserConstructionScript`
  (`parent.UserConstructionScript`))